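; BP_Enemy is an enemy that turns to face the third-person player and performs a heavy attack when they get close.
; Entering the detection Sphere starts a looping timer that interpolates yaw toward the player, and any end overlap clears it.
; The player entering Attack_Sphere prints a debug string and, if CanAttack, plays the heavy attack montage.
; A DoOnce gates the attack, resetting after a short delay once the montage completes or is interrupted.
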(event `self.Sphere.OnComponentBeginOverlap`
  (params (OverlappedComponent :type "PrimitiveComponent Object Reference") (OtherActor :type "Actor Object Reference") (OtherComp :type "PrimitiveComponent Object Reference") (OtherBodyIndex :type Integer) (bFromSweep :type Boolean) (SweepResult :type "HitResult Structure (by ref)"))
  (bind _asbp_third_person_character (cast `/Game/ThirdPerson/Blueprints/BP_ThirdPersonCharacter` OtherActor))
  (set `self.Ref_Character` _asbp_third_person_character)
  (bind _returnvalue (`KismetSystemLibrary.K2_SetTimerDelegate` (delegate `Turn`) 0.01 true))
  (set `self.FaceTimer` _returnvalue))

(event `Turn`
  (bind (_returnvalue_roll _returnvalue_pitch _returnvalue_yaw) (`KismetMathLibrary.BreakRotator` (`KismetMathLibrary.RInterpTo` (`self.K2_GetActorRotation`) (`KismetMathLibrary.FindLookAtRotation` (`self.K2_GetActorLocation`) (`self.K2_GetActorLocation` (`self.Ref_Character`))) (`GameplayStatics.GetWorldDeltaSeconds`))))
  (`self.K2_SetActorRotation` (`KismetMathLibrary.MakeRotator` 0.0 0.0 _returnvalue_yaw)))

(event `self.Sphere.OnComponentEndOverlap`
  (params (OverlappedComponent :type "PrimitiveComponent Object Reference") (OtherActor :type "Actor Object Reference") (OtherComp :type "PrimitiveComponent Object Reference") (OtherBodyIndex :type Integer))
  (`KismetSystemLibrary.K2_ClearAndInvalidateTimerHandle` (`self.FaceTimer`)))

(event `self.Attack_Sphere.OnComponentBeginOverlap`
  (params (OverlappedComponent :type "PrimitiveComponent Object Reference") (OtherActor :type "Actor Object Reference") (OtherComp :type "PrimitiveComponent Object Reference") (OtherBodyIndex :type Integer) (bFromSweep :type Boolean) (SweepResult :type "HitResult Structure (by ref)"))
  (cast `/Game/ThirdPerson/Blueprints/BP_ThirdPersonCharacter` OtherActor)
  (`KismetSystemLibrary.PrintString` "KILLING MYSELF IN REAL TIME")
  (if (`self.CanAttack`)
    (`self.HeavyAttack`)))

(event `HeavyAttack`
  (`/Engine/EditorBlueprintResources/StandardMacros.DoOnce` false :!label _label
    (:`Completed`
      (set `self.CanAttack` false)
      (`|PlayMontage` (`self.Mesh`) "/Game/Sword_Animations/Animations/Sequence1/02_Attack/01_Combo_Attack_01/AM_HeavyAttack.AM_HeavyAttack"
        (:`OnCompleted`
          _)
        (:`OnInterrupted`
          _))
      (set `self.CanAttack` true)
      (`KismetSystemLibrary.Delay` 1.0)
      (goto _label :!via `Reset`))))

(fn `UserConstructionScript`)